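; AI controller for the basic enemy that reacts to the player and bait, running BT_BasicEnemy on possess.
; Unless stunned, target perception updates write player sensing to CanSeePlayer, and bait sensing and location to IsInvestigating and TargetLocation for the tree.
; Any player update, gained or lost, plays the Shocking montage unless already chasing.
; An older noise-tag perception loop remains disconnected.
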(event OnPerceptionUpdated(AIPerception)
  (params (UpdatedActors :type Array%20of%20Actor%20Object%20References)))

(event OnTargetPerceptionUpdated(AIPerception)
  (params (Actor :type Actor%20Object%20Reference) (Stimulus :type AI%20Stimulus%20Structure))
  (bind (_age _expirationage _strength _stimuluslocation _receiverlocation _tag _bsuccessfullysensed) (Utilities|Struct|BreakAIStimulus Stimulus))
  (if (not (ScalableFloat|GetValueasBool (AI|GetBlackboard 0) (Utilities|Name|MakeLiteralName "IsStun")))
    (Utilities|Casting|CastToBP_ThirdPersonCharacter Actor
      (:then
        (AI|Components|Blackboard|SetValueasBool (AI|GetBlackboard 0) (Utilities|Name|MakeLiteralName "CanSeePlayer") (.bSuccessfullySensed (Utilities|Struct|BreakAIStimulus Stimulus)))
        (if (not (ScalableFloat|GetValueasBool (AI|GetBlackboard 0) (Utilities|Name|MakeLiteralName "isChasing")))
          (Animation|Montage|PlayMontage (Variables|/Script/Engine.Character|GetMesh (Variables|Default|GetAs%20BP%20Basic%20Enemy)) "/Game/Animations/Shocking.Shocking")))
      (:CastFailed
        (Utilities|Casting|CastToBP_Bait Actor)
        (AI|Components|Blackboard|SetValueasBool (AI|GetBlackboard 0) (Utilities|Name|MakeLiteralName "IsInvestigating") _bsuccessfullysensed)
        (AI|Components|Blackboard|SetValueasVector (AI|GetBlackboard 0) (Utilities|Name|MakeLiteralName "TargetLocation") _stimuluslocation)))))

(event EventBeginPlay)

(event EventTick
  (params (DeltaSeconds :type Float%20%28single-precision%29)))

(event EventPossess
  (params (PossessedPawn :type Pawn%20Object%20Reference))
  (bind _asbp_basic_enemy (Utilities|Casting|CastToBP_BasicEnemy (Pawn|GetControlledPawn)))
  (Variables|Default|SetAs%20BP%20Basic%20Enemy _asbp_basic_enemy)
  (AI|RunBehaviorTree "/Game/AI/BT_BasicEnemy.BT_BasicEnemy"))

(fn ConstructionScript)