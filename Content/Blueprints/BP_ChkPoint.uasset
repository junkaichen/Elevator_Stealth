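; Checkpoint actor that sets the player's respawn point when a BP_ThirdPersonCharacter overlaps it.
; On overlap it passes its checkpoint name and RespawnPoint location to the level's GameEventManger, found on BeginPlay.
; If that call returns true, a UI_ObjectLight widget label shows a confirmation for a few seconds.
; Tick spins the Checkpoint component in pitch and bobs it with a cosine offset added to its current position each frame.
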(event Custom|ShowTxt
  (CallFunction|SetLabel "Check Point Set!")
  (Utilities|FlowControl|Delay 5.0)
  (CallFunction|SetLabel))

(event EventBeginPlay
  (Utilities|FlowControl|Sequence
    (:then_0
      (bind _asui_object_light (Utilities|Casting|CastToUI_ObjectLight (UserInterface|GetUserWidgetObject (Variables|Default|GetTxt))))
      (Variables|Default|SetLabel _asui_object_light))
    (:then_1
      (bind _returnvalue (Actor|GetActorOfClass "/Game/Blueprints/GameEventManger.GameEventManger_C"))
      (Utilities|IsValid _returnvalue
        (:Is%20Valid
          (Variables|Default|SetGameEventManager _returnvalue))))))

(event Collision|EventActorBeginOverlap
  (params (OtherActor :type Actor%20Object%20Reference))
  (Utilities|Casting|CastToBP_ThirdPersonCharacter OtherActor)
  (bind _rslt (Default|SetCheckPointFunc (Variables|Default|GetGameEventManager) (Variables|Default|GetCheckPointName) (Transformation|GetWorldLocation (Variables|Default|GetRespawnPoint))))
  (if _rslt
    (CallFunction|ShowTxt)))

(event EventTick
  (params (DeltaSeconds :type Float%20%28single-precision%29))
  ;[1 1 1] Floating animation
  (Transformation|AddLocalRotation (Variables|Default|Getcheckpoint) (Math|Rotator|MakeRotator 0.0 (* DeltaSeconds 15.0) 0.0) false false)
  (bind _output_get (Variables|Default|SetMovement (+ DeltaSeconds (Variables|Default|GetMovement))))
  (Transformation|SetRelativeLocation (Variables|Default|Getcheckpoint) (+ (Math|Vector|MakeVector 0.0 0.0 (* (Math|Trig|Cos(Radians) _output_get) 0.2)) (Variables|/Script/Engine.SceneComponent|GetRelativeLocation (Variables|Default|Getcheckpoint))) false false))

(fn ConstructionScript)

(fn SetLabel
  (params (Content :type Text))
  (bind _label (Variables|Default|GetLabel))
  (Utilities|IsValid _label
    (:Is%20Valid
      (Variables|/Game/Blueprints/UI_ObjectLight.UI_ObjectLight_C|SetTagContent _label Content))))