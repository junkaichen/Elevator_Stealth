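; BP_Ghost is a ghost Blueprint with a text label showing its enemy state text, which is set in the construction script.
; BeginPlay caches the player's BP_ThirdPersonCharacter.
; TextFacingToCamera uses that reference to yaw the label toward the first child of the camera boom, flattening the direction to the horizontal plane.
; No graph shown here calls that function.
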(event EventBeginPlay
  (bind _asbp_third_person_character (Utilities|Casting|CastToBP_ThirdPersonCharacter (Game|Player|GetPlayerPawn 0)))
  (Variables|Default|SetAs%20BP%20Third%20Person%20Character _asbp_third_person_character))

(fn ConstructionScript
  (Rendering|Components|TextRender|SetText (Variables|Default|GetTextRender) (Variables|Default|GetEnemyStateText)))

(fn TextFacingtoCamera
  (Transformation|SetWorldRotation (Variables|Default|GetTextRender) (Math|Conversions|RotationFromXVector (Math|Vector|RotateVector (Math|Vector|Normalize (* (- (Transformation|GetWorldLocation (Components|GetChildComponent (Variables|/Game/ThirdPerson/Blueprints/BP_ThirdPersonCharacter.BP_ThirdPersonCharacter_C|GetCameraBoom (Variables|Default|GetAs%20BP%20Third%20Person%20Character)) 0)) (Transformation|GetActorLocation)) "1.000000,1.000000,0")) "0, 0, 0")) false false))