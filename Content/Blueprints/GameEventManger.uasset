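; Game event manager actor that relays chat commands and content through event dispatchers and tracks player checkpoints.
; Binding to its own object trigger, it assigns an unclaimed chat user ID to the first unnamed BP_ChatEnemy or BP_Pikmin, allowing one claim per user until removed.
; Checkpoint changes store a respawn location, and player death teleports the character there and resets it.
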(event Custom|TriggerFunction
  ;[1 1 1] Trigger the objects
  (Default|CallObjectTrigger "" (Variables|Default|GetObjId)))

(event Custom|TriggerFunction_Cmd
  (params (UserId :type String) (ObjId :type String))
  ;[1 1 1] Chat input command
  (if (Utilities|Enum|NotEqual(Enum) (Utilities|String|Trim ObjId) "")
    (Default|CallObjectTrigger UserId ObjId)))

(event Custom|TriggerChatContent
  (params (UserId :type String) (Content :type String))
  ;[1 1 1] Chat input action
  (Default|CallChatContentTrigger UserId Content))

(event Custom|RemoveName
  (params (UserId :type String))
  ;[1 1 1] Remove User name from list
  (if (!= (Utilities|Array|FindItem (Variables|Default|GetChatNames) UserId) -1)
    (Utilities|Array|RemoveItem (Variables|Default|GetChatNames) UserId)))

(event Custom|ChatEnemyNameSetting
  (params (UserId :type String) (ObjId :type String))
  ;[1 1 1] Pick enemy/pikmin for naming
  (if (< (Utilities|Array|FindItem (Variables|Default|GetChatNames) UserId) 0)
    (switch string ObjId
      (:enemy
        (bind _outactors (Actor|GetAllActorsOfClass "/Game/Blueprints/MapObject/BP_ChatEnemy.BP_ChatEnemy_C"))
        (bind _array_element (Utilities|Array|ForEachLoopwithBreak _outactors :!label _label)
          (:LoopBody
            (if (Utilities|Enum|Equal(Enum) (Variables|/Game/Blueprints/MapObject/BP_ChatEnemy.BP_ChatEnemy_C|GetUserId _array_element) "")
              (Development|PrintString (Utilities|GetObjectName _array_element))
              (Default|SetUserId _array_element UserId)
              (Utilities|Array|Add (Variables|Default|GetChatNames) UserId)
              (goto _label Break)))))
      (:friend
        (bind _outactors_2 (Actor|GetAllActorsOfClass "/Game/Blueprints/Pikmin/BP_Pikmin.BP_Pikmin_C"))
        (bind _array_element_2 (Utilities|Array|ForEachLoopwithBreak _outactors_2 :!label _label_2)
          (:LoopBody
            (if (Utilities|Enum|Equal(Enum) (Variables|/Game/Blueprints/Pikmin/BP_Pikmin.BP_Pikmin_C|GetUserId _array_element_2) "")
              (Variables|/Game/Blueprints/Pikmin/BP_Pikmin.BP_Pikmin_C|SetUserId _array_element_2 UserId)
              (Utilities|Array|Add (Variables|Default|GetChatNames) UserId)
              (goto _label_2 Break))))))))

(event Custom|PlayerDeath
  (Transformation|SetActorLocation (Game|GetPlayerCharacter 0) (Variables|CheckPoints|GetRespawnLocation) false true)
  (bind _asbp_third_person_character (Utilities|Casting|CastToBP_ThirdPersonCharacter (Game|GetPlayerCharacter 0)))
  (Default|ResetCharacter _asbp_third_person_character))

(event Custom|SetCheckPoint
  (params (CheckPoint :type String) (Location :type Vector))
  (if (not (Utilities|Enum|Equal(Enum) CheckPoint (Variables|CheckPoints|GetCurrentChkPnt)))
    (Variables|CheckPoints|SetCurrentChkPnt CheckPoint)
    (Variables|CheckPoints|SetRespawnLocation Location)
    (Development|PrintString "CheckPointSet" true true "(R=0.179082,G=1.000000,B=0.000000,A=1.000000)")))

(event EventBeginPlay
  (EventDispatchers|BindEventtoObjectTrigger (delegate Custom|ChatEnemyNameSetting)))

(fn ConstructionScript)