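; BP_BasicEnemy is an AI enemy that melee-attacks the player and displays its awareness state as floating text.
; MeleeAttack plays the attack montage and, if the player is close, sets the JustKillPlayer blackboard key and calls HitByEnemy on the player.
; Tick picks an alert, searching or idle symbol from blackboard sight and chase keys plus the AI controller's hearing data.
; The text turns horizontally to face the player's camera.
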(event EventBeginPlay
  (bind _asbp_third_person_character (Utilities|Casting|CastToBP_ThirdPersonCharacter (Game|Player|GetPlayerPawn 0)))
  (Variables|Default|SetAs%20BP%20Third%20Person%20Character _asbp_third_person_character))

(event EventTick
  (params (DeltaSeconds :type Float%20%28single-precision%29))
  ;[1 1 1] Set Eenemy State TEXT
  (if (ScalableFloat|GetValueasBool (AI|GetBlackboard 0) (Utilities|Name|MakeLiteralName "CanSeePlayer"))
    (bind _output_get (Variables|Default|SetEnemyStateText "!"))
    (Rendering|Components|TextRender|SetText (Variables|Default|GetTextRender) _output_get)
    (elif (ScalableFloat|GetValueasBool (AI|GetBlackboard 0) (Utilities|Name|MakeLiteralName "Ischasing"))
      (bind _output_get_2 (Variables|Default|SetEnemyStateText "?"))
      (Rendering|Components|TextRender|SetText (Variables|Default|GetTextRender) _output_get_2)
      (else
        (Variables|Default|SetEnemyStateText "(^_^ )")
        (bind _asbp_basic_enemy_aicontroller (Utilities|Casting|CastToBP_BasicEnemyAIController (Pawn|GetController)))
        (if (> (Variables|/Game/AI/BP_BasicEnemyAIController.BP_BasicEnemyAIController_C|GetNoiseCounter _asbp_basic_enemy_aicontroller) 0)
          (if (Variables|/Game/AI/BP_BasicEnemyAIController.BP_BasicEnemyAIController_C|GetInHearingRange _asbp_basic_enemy_aicontroller)
            (bind _output_get_3 (Variables|Default|SetEnemyStateText "?"))))
        (Rendering|Components|TextRender|SetText (Variables|Default|GetTextRender) _output_get_3))))
  (CallFunction|TextFacingtoCamera))

(event EventMeleeAttack
  ;[1 1 1] Enemy Attack Player
  (Animation|Montage|PlayMontage (Variables|Character|GetMesh) "/Game/Animations/Attack.Attack" 1.5
    (:then
      (if (< (Transformation|GetDistanceTo (Variables|Default|GetAs%20BP%20Third%20Person%20Character) self) 2.5e+02)
        (AI|Components|Blackboard|SetValueasBool (AI|GetBlackboard 0) (Utilities|Name|MakeLiteralName "JustKillPlayer") true)
        (Default|HitbyEnemy (Variables|Default|GetAs%20BP%20Third%20Person%20Character))))))

(fn ConstructionScript
  (Rendering|Components|TextRender|SetText (Variables|Default|GetTextRender) (Variables|Default|GetEnemyStateText)))

(fn TextFacingtoCamera
  (Transformation|SetWorldRotation (Variables|Default|GetTextRender) (Math|Conversions|RotationFromXVector (Math|Vector|RotateVector (Math|Vector|Normalize (* (- (Transformation|GetWorldLocation (Components|GetChildComponent (Variables|/Game/ThirdPerson/Blueprints/BP_ThirdPersonCharacter.BP_ThirdPersonCharacter_C|GetCameraBoom (Variables|Default|GetAs%20BP%20Third%20Person%20Character)) 0)) (Transformation|GetActorLocation)) "1.000000,1.000000,0")) "0, 0, 0")) false false))