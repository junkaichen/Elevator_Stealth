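; Triggerable map object that spawns a basic enemy from behind an animated gate.
; When triggered, a timeline moves the door frame vertically, then an AI enemy with its behavior tree spawns at the gate and receives the configured patrol path.
; After short delays a second timeline moves the frame back.
; A CanSpawn flag blocks retriggering until the whole cycle finishes.
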(event Custom|SpawnFunction
  (bind _closescale (Timeline|ShowDoor PlayFromStart)
    (:Update
      (Transformation|SetRelativeLocation (Variables|Default|GetSM_DoorFrame) (Math|Vector|MakeVector 0.0 0.0 (* _closescale -2.5e+02)) false false))
    (:Finished
      (Utilities|FlowControl|Delay 0.3)
      (bind _returnvalue (AI|SpawnAIFromClass "/Game/Blueprints/BP_BasicEnemy.BP_BasicEnemy_C" "/Game/AI/BT_BasicEnemy.BT_BasicEnemy" (+ (Transformation|GetActorLocation self) "0,0,88.000000") "0, 0,0.000000" false 0))
      (bind _asbp_basic_enemy (Utilities|Casting|CastToBP_BasicEnemy _returnvalue))
      (Variables|/Game/Blueprints/BP_BasicEnemy.BP_BasicEnemy_C|SetPatrolPath _asbp_basic_enemy (Variables|Default|GetPathSetting))
      (Utilities|FlowControl|Delay 0.3)
      (bind _openscale (Timeline|HideDoor PlayFromStart)
        (:Update
          (Transformation|SetRelativeLocation (Variables|Default|GetSM_DoorFrame) (Math|Vector|MakeVector 0.0 0.0 (* _openscale -2.5e+02)) false false))
        (:Finished
          (Variables|Default|SetCanSpawn true))))))

(event EventBeginPlay
  (|CallParentFunction))

(event EventTriggerAction
  (if (Variables|Default|GetCanSpawn)
    (Variables|Default|SetCanSpawn false)
    (CallFunction|SpawnFunction)))

(fn ConstructionScript
  (|CallParentFunction))