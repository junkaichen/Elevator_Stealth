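; Base Blueprint for interactive map objects that respond to object-trigger events, with an empty TriggerAction event as the hook for specific behavior.
; On BeginPlay it finds the GameEventManger actor and binds TriggerEvent to its ObjectTrigger.
; TriggerEvent passes the UserId to TriggerAction when the ObjId comparison against a lowercased ObjId matches.
; A separate IsCloseToPlayer helper, unused here, checks whether player 0's character is within a fixed radius.
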(event Custom|TriggerEvent
  (params (UserId :type String) (ObjId :type String))
  (if (Utilities|Enum|Equal(Enum) ObjId (Utilities|String|ToLower (Variables|Default|GetObjId)))
    (CallFunction|TriggerAction UserId)))

(event Custom|TriggerAction
  (params (UserId :type String)))

(event EventBeginPlay
  (bind _returnvalue (Actor|GetActorOfClass "/Game/Blueprints/GameEventManger.GameEventManger_C"))
  (Utilities|IsValid _returnvalue
    (:Is%20Valid
      (EventDispatchers|BindEventtoObjectTrigger _returnvalue (delegate Custom|TriggerEvent)))))

(fn ConstructionScript)

(fn IsClosetoPlayer
  (return (< (Math|Vector|Distance(Vector) (Transformation|GetActorLocation (Game|GetPlayerCharacter 0)) (Transformation|GetActorLocation)) 1e+03)))