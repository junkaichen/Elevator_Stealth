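; BP_LightObj is a map object light that switches on and off when triggered.
; On BeginPlay it sets the PointLight to full or zero intensity from the Open flag, then calls the parent.
; TriggerAction flips Open, while LightUp forces it on.
; Both run LightChange, which plays separate open and close timelines to animate the intensity.
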(event Custom|LightChange
  (bind _pointlight (Variables|Default|GetPointLight))
  ;[1 1 1] Change
  (if (Variables|Default|GetOpen)
    (bind _openscale (Timeline|OpenTimer PlayFromStart)
      (:Update
        (Rendering|Components|Light|SetIntensity _pointlight (* _openscale 5e+04))))
    (else
      (bind _closescale (Timeline|CloseTimer PlayFromStart)
        (:Update
          (Rendering|Components|Light|SetIntensity _pointlight (* _closescale 5e+04)))))))

(event Custom|LightInitial
  (bind _pointlight (Variables|Default|GetPointLight))
  ;[1 1 1] Initial Setting
  (if (Variables|Default|GetOpen)
    (Rendering|Components|Light|SetIntensity _pointlight 5e+04)
    (else
      (Rendering|Components|Light|SetIntensity _pointlight 0.0))))

(event Custom|LightUp
  ;[1 1 1] Open za lighto
  (Variables|Default|SetOpen true)
  (CallFunction|LightChange))

(event EventBeginPlay
  (CallFunction|LightInitial)
  (|CallParentFunction))

(event EventTriggerAction
  ;[1 1 1] Action when triggered
  (Variables|Default|SetOpen (not (Variables|Default|GetOpen)))
  (CallFunction|LightChange))

(fn ConstructionScript
  (|CallParentFunction))