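; BP_ChatEnemy is an enemy tied to a chat UserId that shows that user's messages on its ChatUI widget.
; It listens to GameEventManger's chat trigger, stores matching content until the DisplayContent timeline finishes, and hands itself to UI_EnemyChat.
; Tick shows the widget only while the player is near, testing horizontal and vertical distance separately.
; On destruction it removes its UserId from the manager through RemoveName.
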(event Custom|SetUserId
  (params (UserId :type String))
  (Variables|Default|SetUserId UserId))

(event Custom|ChatContent
  (params (UserId :type String) (Content :type String))
  (if (Utilities|Enum|Equal(Enum) UserId (Variables|Default|GetUserId))
    (Development|PrintString Content)
    (Variables|Default|SetContent Content)
    (Timeline|DisplayContent PlayFromStart
      (:Finished
        (Variables|Default|SetContent "")))))

(event Custom|RemoveName
  (params (DestroyedActor :type Actor%20Object%20Reference))
  (bind _returnvalue (Actor|GetActorOfClass "/Game/Blueprints/GameEventManger.GameEventManger_C"))
  (Utilities|IsValid _returnvalue
    (:Is%20Valid
      (Default|RemoveName _returnvalue (Variables|Default|GetUserId)))))

(event EventBeginPlay
  (bind _returnvalue (Game|GetPlayerCharacter 0))
  (|CallParentFunction)
  (Utilities|FlowControl|Sequence
    (:then_0
      (Game|BindEventtoOnDestroyed (delegate Custom|RemoveName)))
    (:then_1
      (bind _returnvalue_2 (Actor|GetActorOfClass "/Game/Blueprints/GameEventManger.GameEventManger_C"))
      (Utilities|IsValid _returnvalue_2
        (:Is%20Valid
          (EventDispatchers|BindEventtoChatContentTrigger _returnvalue_2 (delegate Custom|ChatContent))
          (bind _asui_enemy_chat (Utilities|Casting|CastToUI_EnemyChat (UserInterface|GetUserWidgetObject (Variables|Default|GetChatUI))))
          (Variables|/Game/Blueprints/MapObject/UI_EnemyChat.UI_EnemyChat_C|SetChatEnemy _asui_enemy_chat self))))
    (:then_2
      (Utilities|IsValid _returnvalue
        (:Is%20Valid
          (Variables|Default|SetPlayerCharacter _returnvalue))))))

(event EventTick
  (params (DeltaSeconds :type Float%20%28single-precision%29))
  (bind _rslt (CallFunction|IsClosetoPlayer))
  (Rendering|SetVisibility (Variables|Default|GetChatUI) _rslt false))

(fn ConstructionScript
  (|CallParentFunction))

(fn IsClosetoPlayer
  (bind _returnvalue (Transformation|GetActorLocation))
  (bind _playercharacter (Variables|Default|GetPlayerCharacter))
  (bind _returnvalue_2 (Transformation|GetActorLocation _playercharacter))
  (Utilities|IsValid (Variables|Default|GetPlayerCharacter)
    (:Is%20Valid
      (return (and (< (Math|Vector|Distance(Vector) (Math|Vector|MakeVector (.x _returnvalue_2) (.y _returnvalue_2) 0.0) (Math|Vector|MakeVector (.x _returnvalue) (.y _returnvalue) 0.0)) 4e+03) (< (Math|Float|Absolute(Float) (- (.z _returnvalue_2) (.z _returnvalue))) 5e+02))))
    (:Is%20Not%20Valid
      (return false))))