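; BP_Trap is a single-use map trap that kills the first BP_BasicEnemy to overlap it while the player is nearby.
; Tick toggles CanUse from the player's distance to the trap.
; A valid overlap plays a bone-pile sound, ragdolls the enemy and sets IsDead on its blackboard.
; After a short delay, it destroys the enemy, if still valid, along with the trap's Niagara component.
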(event EventBeginPlay
  (|CallParentFunction) ; This node is disabled and will not be called.\nDrag off pins to build functionality.
)

(event Collision|EventActorBeginOverlap
  (params (OtherActor :type Actor%20Object%20Reference))
  (bind _asbp_basic_enemy (Utilities|Casting|CastToBP_BasicEnemy OtherActor))
  (if (and (not (Variables|Default|GetIsUsed)) (Variables|Default|GetCanUse))
    (Variables|Default|SetIsUsed true)
    (Variables|Default|SetEnemy _asbp_basic_enemy)
    (Audio|PlaySoundatLocation "/Game/Audio/Environment/BonePile.BonePile" (Transformation|GetActorLocation) "0, 0, 0" 1.0 1.0 0.0 0 0 0 0)
    (Collision|SetCollisionEnabled (Variables|/Script/Engine.Character|GetMesh _asbp_basic_enemy) "QueryAndPhysics")
    (Physics|SetSimulatePhysics (Variables|/Script/Engine.Character|GetMesh _asbp_basic_enemy) true)
    (AI|Components|Blackboard|SetValueasBool (AI|GetBlackboard _asbp_basic_enemy) (Utilities|Name|MakeLiteralName "IsDead") true)
    (Utilities|FlowControl|Delay 1.58)
    (Utilities|IsValid (Variables|Default|GetEnemy)
      (:Is%20Valid
        (Actor|DestroyActor (Variables|Default|GetEnemy))
        (Components|DestroyComponent (Variables|Default|GetNiagara))))))

(event EventTick
  (params (DeltaSeconds :type Float%20%28single-precision%29))
  (if (< (Math|Vector|Distance(Vector) (Transformation|GetActorLocation (Game|GetPlayerCharacter 0)) (Transformation|GetActorLocation)) 6e+02)
    (Variables|Default|SetCanUse true)
    (else
      (Variables|Default|SetCanUse false))))

(fn ConstructionScript
  (|CallParentFunction))