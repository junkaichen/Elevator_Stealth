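; BP_HidingSpot is a map object that, when triggered, removes itself and clears the player character's Hidden flag.
; Its construction script labels CommandText with "!" followed by the object's ObjId.
; Each Tick rotates that text toward the first player controller's location.
; TriggerAction destroys the actor, then casts the player character to BP_ThirdPersonCharacter and sets Hidden to false.
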(event EventBeginPlay
  (|CallParentFunction) ; This node is disabled and will not be called.\nDrag off pins to build functionality.
)

(event Collision|EventActorBeginOverlap
  (params (OtherActor :type Actor%20Object%20Reference)))

(event EventTick
  (params (DeltaSeconds :type Float%20%28single-precision%29))
  (Transformation|SetWorldRotation (Variables|Default|GetCommandText) (Math|Rotator|FindLookatRotation (Transformation|GetActorLocation) (Transformation|GetActorLocation (Game|GetPlayerController 0))) false false))

(event EventTriggerAction
  (Actor|DestroyActor)
  (bind _asbp_third_person_character (Utilities|Casting|CastToBP_ThirdPersonCharacter (Game|GetPlayerCharacter 0)))
  (Variables|/Game/ThirdPerson/Blueprints/BP_ThirdPersonCharacter.BP_ThirdPersonCharacter_C|SetHidden _asbp_third_person_character false))

(fn ConstructionScript
  (|CallParentFunction)
  (Rendering|Components|TextRender|SetText (Variables|Default|GetCommandText) (Utilities|Text|ToText(String) (Utilities|String|Append "!" (Variables|Default|GetObjId)))))