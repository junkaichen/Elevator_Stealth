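; Map actor that runs repeating timed chat votes between a random skill from SkillList and one from SkillListBad.
; After a short delay, it shows UI_Voting and counts L/R commands from TriggerEvent during a timeline-driven countdown, logging votes to chat.
; When time ends, it sends the winning skill's command, with random tie-breaks, to GameEventManager, then starts the next round.
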(event Custom|Voting
  (bind _ui (Variables|Default|GetUI))
  (bind _ui_2 (Variables|Default|GetUI))
  (bind _ui_3 (Variables|Default|GetUI))
  (Utilities|FlowControl|Delay 5.0)
  (Variables|Default|SetLeftSel (Math|Random|RandomInteger (Utilities|Array|Length (Variables|Default|GetSkillList))))
  (Variables|Default|SetRightSel (Math|Random|RandomInteger (Utilities|Array|Length (Variables|Default|GetSkillList_Bad))))
  (Development|PrintString (Utilities|String|Append (.skillname (Utilities|Array|Get(acopy) (Variables|Default|GetSkillList) (Variables|Default|GetLeftSel))) " VS " (.skillname (Utilities|Array|Get(acopy) (Variables|Default|GetSkillList_Bad) (Variables|Default|GetRightSel)))))
  (Default|SetVoteTopic _ui (.skillname (Utilities|Array|Get(acopy) (Variables|Default|GetSkillList) (Variables|Default|GetLeftSel))) (.skillname (Utilities|Array|Get(acopy) (Variables|Default|GetSkillList_Bad) (Variables|Default|GetRightSel))))
  (UserInterface|Viewport|AddtoViewport _ui 0)
  (bind _output_get (Variables|Vote|SetLeftVoteNum 0))
  (bind _output_get_2 (Variables|Vote|SetRightVoteNum 0))
  (Variables|Default|SetStartVoting true)
  (Default|ChangeVoteValue _ui_2 _output_get _output_get_2)
  (Default|LeftUser _ui_2)
  (Default|RightUser _ui_2)
  (bind _countdown (Timeline|VoteTime PlayFromStart)
    (:Update
      (Default|SetTimer _ui_3 (Utilities|Text|ToText(Float) _countdown "HalfToEven" false true 1 324 1 1)))
    (:Finished
      (Default|SetTimer _ui_3)
      (Widget|RemovefromParent (Variables|Default|GetUI))
      (Variables|Default|SetStartVoting false)
      (CallFunction|AfterVote)
      (CallFunction|Voting))))

(event Custom|UserVote
  (params (Cmd :type String) (UserId :type String))
  (bind _returnvalue (Utilities|Text|ToText(String) UserId))
  (bind _ui (Variables|Default|GetUI))
  ;[1 1 1] The action when user voting
  (switch string Cmd
    (:L
      (Variables|Vote|SetLeftVoteNum (+ (Variables|Vote|GetLeftVoteNum) 1))
      (Default|LeftUser _ui _returnvalue)
      (CallFunction|SendLog UserId (Utilities|Array|Get(acopy) (Variables|Default|GetSkillList) (Variables|Default|GetLeftSel))))
    (:R
      (Variables|Vote|SetRightVoteNum (+ (Variables|Vote|GetRightVoteNum) 1))
      (Default|RightUser _ui _returnvalue)
      (CallFunction|SendLog UserId (Utilities|Array|Get(acopy) (Variables|Default|GetSkillList) (Variables|Default|GetRightSel)))))
  (Default|ChangeVoteValue _ui (Variables|Vote|GetLeftVoteNum) (Variables|Vote|GetRightVoteNum)))

(event Custom|AfterVote
  (bind _leftvotenum (Variables|Vote|GetLeftVoteNum))
  (bind _rightvotenum (Variables|Vote|GetRightVoteNum))
  (bind _gameeventmanager (Variables|Default|GetGameEventManager))
  (if (!= _leftvotenum _rightvotenum)
    (if (> _leftvotenum _rightvotenum)
      (CallFunction|SetCommand (Variables|Default|GetLeftSel) (Variables|Default|GetSkillList) :!label _label)
      (else
        (CallFunction|SetCommand (Variables|Default|GetRightSel) (Variables|Default|GetSkillList_Bad) :!label _label_2)))
    (elif (< (Math|Random|RandomInteger 2) 1)
      (goto _label_2)
      (else
        (goto _label))))
  (Utilities|IsValid _gameeventmanager
    (:Is%20Valid
      (Default|CallObjectTrigger _gameeventmanager "" (Variables|Default|GetRsltCmd)))))

(event EventBeginPlay
  (|CallParentFunction)
  (bind _returnvalue (UserInterface|CreateWidget "/Game/Blueprints/MapObject/UI_Voting.UI_Voting_C"))
  (Variables|Default|SetUI _returnvalue)
  (Utilities|FlowControl|Sequence
    (:then_0
      (CallFunction|Voting))
    (:then_1
      (bind _returnvalue_2 (Actor|GetActorOfClass "/Game/Blueprints/GameEventManger.GameEventManger_C"))
      (Utilities|IsValid _returnvalue_2
        (:Is%20Valid
          (Variables|Default|SetGameEventManager _returnvalue_2))))))

(event EventTriggerEvent
  (params (UserId :type String) (ObjId :type String))
  ;[1 1 1] Get the chat command
  (if (Variables|Default|GetStartVoting)
    (for _array_element (Variables|Default|GetCmdList)
      (if (Utilities|Enum|Equal(Enum) _array_element ObjId)
        (CallFunction|UserVote ObjId UserId)))))

(fn ConstructionScript
  (|CallParentFunction))

(fn SetCommand
  (params (Index :type Integer) (Array :type Array%20of%20Skill%20Data%20Structures))
  (Variables|Default|SetRsltCmd (.skillcommand (Utilities|Array|Get(acopy) Array Index))))

(fn SendLog
  (params (UserId :type String) (Skill :type Skill%20Data%20Structure))
  (Default|AddChatLog (Variables|Default|GetGameEventManager) (Utilities|String|Append UserId " vote for " (.SkillName (Utilities|Struct|BreakSkillData Skill)))))