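; Interactable map door that toggles open and closed when triggered, then locks out further use during a short cooldown.
; Separate open and close timelines drive the door's yaw, and BeginPlay snaps it to match its initial Open state.
; Each toggle posts a colored chat line naming user and object through the GameEventManger actor.
; Tick shows the object ID on a widget label while the player is near and the door is usable.
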(event Custom|DoorMovement
  (bind _door (Variables|Default|GetDoor))
  (if (Variables|Default|GetOpen)
    (bind _openscale (Timeline|OpenTimer PlayFromStart)
      (:Update
        (Transformation|SetRelativeRotation _door (Math|Rotator|MakeRotator 0.0 0.0 (* _openscale 9e+01)) false false)))
    (else
      (bind _closescale (Timeline|CloseTimer PlayFromStart)
        (:Update
          (Transformation|SetRelativeRotation _door (Math|Rotator|MakeRotator 0.0 0.0 (* _closescale 9e+01)) false false))))))

(event Custom|CoolDown
  (Utilities|FlowControl|Delay 5.0)
  (Variables|Default|SetCanUse true))

(event Custom|DoorInitial
  (bind _door (Variables|Default|GetDoor))
  (if (Variables|Default|GetOpen)
    (Transformation|SetRelativeRotation _door (Math|Rotator|MakeRotator 0.0 0.0 9e+01) false false)
    (else
      (Transformation|SetRelativeRotation _door (Math|Rotator|MakeRotator 0.0 0.0 0.0) false false))))

(event EventBeginPlay
  (CallFunction|DoorInitial)
  (|CallParentFunction)
  (Utilities|FlowControl|Sequence
    (:then_0
      (bind _returnvalue (Actor|GetActorOfClass "/Game/Blueprints/GameEventManger.GameEventManger_C"))
      (Variables|Default|SetGameEventManager _returnvalue))
    (:then_1
      (bind _asui_object_light (Utilities|Casting|CastToUI_ObjectLight (UserInterface|GetUserWidgetObject (Variables|Default|GetLabelWidget))))
      (Variables|Default|SetLabel _asui_object_light))))

(event EventTick
  (params (DeltaSeconds :type Float%20%28single-precision%29))
  (bind _newparam (CallFunction|IsClosetoPlayer))
  (if (and _newparam (Variables|Default|GetCanUse))
    (CallFunction|SetLabel (Utilities|Text|ToText(String) (Utilities|String|Append "!" (Variables|Default|GetObjId))))
    (else
      (CallFunction|SetLabel))))

(event EventTriggerAction
  (params (UserId :type String))
  (if (Variables|Default|GetCanUse)
    (CallFunction|SetLog UserId)
    (Variables|Default|SetCanUse false)
    (Variables|Default|SetOpen (not (Variables|Default|GetOpen)))
    (CallFunction|DoorMovement)
    (CallFunction|CoolDown)))

(fn ConstructionScript
  (|CallParentFunction))

(fn SetLabel
  (params (Content :type Text))
  (bind _label (Variables|Default|GetLabel))
  (Utilities|IsValid _label
    (:Is%20Valid
      (Variables|/Game/Blueprints/UI_ObjectLight.UI_ObjectLight_C|SetTagContent _label Content))))

(fn SetLog
  (params (UserId :type String))
  (bind _gameeventmanager (Variables|Default|GetGameEventManager))
  (Utilities|IsValid _gameeventmanager
    (:Is%20Valid
      (Default|AddChatLog _gameeventmanager (Utilities|String|Append "<YellowTxt>" UserId "</>" " switched " "<BlueTxt>" (Variables|Default|GetObjId) "</> !")))))