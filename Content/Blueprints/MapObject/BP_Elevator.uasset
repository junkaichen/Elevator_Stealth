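; Elevator actor that carries the player between floors, ping-ponging one level per trip, either on character overlap or automatically after a Tick-driven cooldown.
; The construction script builds the floor list from child billboards sorted by trailing name digit, and disables the trigger in automatic mode.
; MoveToCertainFloor closes the rotating door, steps through floors with a custom bidirectional delayed-loop macro driving a timeline lerp and sound, then reopens it.
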(event OnComponentBeginOverlap(TriggerBox)
  (params (OverlappedComponent :type Primitive%20Component%20Object%20Reference) (OtherActor :type Actor%20Object%20Reference) (OtherComp :type Primitive%20Component%20Object%20Reference) (OtherBodyIndex :type Integer) (bFromSweep :type Boolean) (SweepResult :type Hit%20Result%20Structure%20%28by%20ref%29))
  (bind _currentlevel (Variables|Default|GetCurrentLevel))
  ;[1 1 1] Trigger the elevator
  (Utilities|Casting|CastToBP_ThirdPersonCharacter OtherActor)
  (if (== _currentlevel (- (Utilities|Array|Length (Variables|Default|GetBillboardsList)) 1))
    (Variables|Default|SetDirection false)
    (elif (== _currentlevel 0)
      (Variables|Default|SetDirection true)))
  (CallFunction|MovetoCertainFloor (select (Variables|Default|GetDirection) (+ _currentlevel 1) (- _currentlevel 1))))

(event Custom|ChangeDoorStatus
  (params (Open :type Boolean))
  (bind _door (Variables|Default|GetDoor))
  (bind _relativerotation (Variables|/Script/Engine.SceneComponent|GetRelativeRotation _door))
  ;[1 1 1] TODO:: Replace them to open door animations
  (if (!= Open (Variables|Default|GetIsOpened))
    (bind _output_get (Variables|Default|SetStartRotator (Variables|/Script/Engine.SceneComponent|GetRelativeRotation _door)))
    (bind _move (Timeline|Door%20Rotation PlayFromStart)
      (:Update
        (Transformation|SetRelativeRotation _door (Math|Rotator|Lerp(Rotator) _output_get (select Open (Math|Rotator|MakeRotator (.roll _relativerotation) (.pitch _relativerotation) 9e+01) (Math|Rotator|MakeRotator (.roll _relativerotation) (.pitch _relativerotation) 0.0)) _move) false false)
        (Variables|Default|SetIsOpened Open)))))

(event Custom|MoveToCertainFloor
  (params (floor :type Integer))
  (if (Math|Boolean|ANDBoolean (not (Variables|Default|GetRunning)) (>= floor 0) (< floor (Utilities|Array|Length (Variables|Default|GetBillboardsList))))
    (CallFunction|ChangeDoorStatus false)
    (Variables|Default|SetRunning true)
    (Components|Timeline|SetPlayRate (Variables|Default|GetTimeline_0) (/ 1.0 (Variables|Default|GetMoveToNextLevelLength)))
    (bind _index (Utilities|RealforLoopwithDelay (select (< (Variables|Default|GetCurrentLevel) floor) (+ (Variables|Default|GetCurrentLevel) 1) (- (Variables|Default|GetCurrentLevel) 1)) floor (Variables|Default|GetMoveToNextLevelLength))
      (:LoopBody
        (Variables|Default|SetStartLocation (Transformation|GetActorLocation))
        (Variables|Default|SetEndLocation (Utilities|Array|Get(acopy) (Variables|Default|GetLevelLocations) _index))
        (bind _returnvalue (Audio|SpawnSoundatLocation "/Game/Audio/Environment/Elevator.Elevator" (Transformation|GetActorLocation) "0, 0, 0" 1.0 1.0 0.0 0 0))
        (Variables|Default|SetElevatorSound _returnvalue)
        (bind _move (Timeline|Timeline_0 PlayFromStart)
          (:Update
            (Transformation|SetActorLocation (Math|Vector|Lerp(Vector) (Variables|Default|GetStartLocation) (Variables|Default|GetEndLocation) _move) false true))
          (:Finished
            (Variables|Default|SetCurrentLevel (select (< (Variables|Default|GetCurrentLevel) floor) (+ (Variables|Default|GetCurrentLevel) 1) (- (Variables|Default|GetCurrentLevel) 1)))
            (Components|Activation|ToggleActive (Variables|Default|GetElevatorSound)))))
      (:Completed
        ;[1 1 1] End of the event
        (Variables|Default|SetRunning false)
        (CallFunction|ChangeDoorStatus true)))))

(event EventBeginPlay
  (for _array_element (Variables|Default|GetBillboardsList)
    (Utilities|Array|Add (Variables|Default|GetLevelLocations) (Transformation|GetWorldLocation _array_element))
    (CallFunction|ChangeDoorStatus true))
  (Transformation|SetActorLocation (Transformation|GetWorldLocation (Utilities|Array|Get(acopy) (Variables|Default|GetBillboardsList) (Variables|Default|GetCurrentLevel))) false true)
  (Variables|Default|SetCoolDownRemaining (Variables|Default|GetCoolDown)))

(event EventTick
  (params (DeltaSeconds :type Float%20%28single-precision%29))
  (bind _currentlevel (Variables|Default|GetCurrentLevel))
  (if (and (Variables|Default|GetAutomaticalMoving) (not (Variables|Default|GetRunning)))
    (if (> (Variables|Default|GetCoolDownRemaining) 0.0)
      (Variables|Default|SetCoolDownRemaining (- (Variables|Default|GetCoolDownRemaining) DeltaSeconds))
      (else
        (Variables|Default|SetCoolDownRemaining (Variables|Default|GetCoolDown))
        (if (== _currentlevel (- (Utilities|Array|Length (Variables|Default|GetBillboardsList)) 1))
          (Variables|Default|SetDirection false)
          (elif (== _currentlevel 0)
            (Variables|Default|SetDirection true)))
        (CallFunction|MovetoCertainFloor (select (Variables|Default|GetDirection) (+ _currentlevel 1) (- _currentlevel 1)))))))

(fn ConstructionScript
  (Utilities|FlowControl|Sequence
    (:then_0
      (|InitBillboards))
    (:then_1
      (if (Variables|Default|GetAutomaticalMoving)
        (Collision|SetCollisionEnabled (Variables|Default|GetTriggerBox) "NoCollision")))))