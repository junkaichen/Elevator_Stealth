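; Map object that, when triggered, temporarily dims a list of rect lights and then brings them back.
; TriggerAction caches each light's intensity, then OffTimeline scales those values through its curve.
; After a fixed delay, OnTimeline drives the lights again from the cached values.
; The restore loop reads the array index from the off loop rather than its own, so every light gets the same cached intensity.
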(event EventBeginPlay
  (|CallParentFunction) ; This node is disabled and will not be called.\nDrag off pins to build functionality.
)

(event EventTriggerAction
  (Utilities|Array|Clear (Variables|Default|GetIntensity))
  (for _array_element (Variables|Default|GetLightLists)
    (Utilities|Array|Add (Variables|Default|GetIntensity) (Variables|/Script/Engine.LightComponentBase|GetIntensity (Variables|/Script/Engine.RectLight|GetRectLightComponent _array_element))))
  (bind _index (Timeline|OffTimeline PlayFromStart)
    (:Update
      (for (_array_element_2 _array_index) (Variables|Default|GetLightLists)
        (Rendering|Components|Light|SetIntensity (Variables|/Script/Engine.Light|GetLightComponent _array_element_2) (* _index (Utilities|Array|Get(acopy) (Variables|Default|GetIntensity) _array_index)))))
    (:Finished
      (Utilities|FlowControl|Delay 8.0)
      (bind _index_2 (Timeline|OnTimeline PlayFromStart)
        (:Update
          (for _array_element_3 (Variables|Default|GetLightLists)
            (Rendering|Components|Light|SetIntensity (Variables|/Script/Engine.Light|GetLightComponent _array_element_3) (* (Utilities|Array|Get(acopy) (Variables|Default|GetIntensity) _array_index) _index_2))))))))

(fn ConstructionScript
  (|CallParentFunction))