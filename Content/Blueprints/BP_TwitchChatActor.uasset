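; Twitch chat actor that connects to a channel and defines prefixed chat commands.
; On BeginPlay it loads credentials, prefix and help text from a JSON file in the project config folder, writing a blank template if missing, then connects.
; IsCommand checks the prefix, and ProcessCommand routes to help message, ping whisper or a test trigger on GameEventManger.
; No graph here calls either function.
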(event EventBeginPlay
  (bind (_token _channel _username _commandprefix _helpmessage) (CallFunction|ReadSettings))
  (CallFunction|SetSettings _token _channel _username _commandprefix _helpmessage))

(fn ConstructionScript)

(fn IsCommand
  (params (message :type String))
  (return (Utilities|String|StartsWith message (Variables|Default|GetcommandPrefix))))

(fn ProcessCommand
  (params (Command :type String) (UserName :type String))
  (bind _username (Variables|Default|Getusername))
  (switch string (Utilities|String|ToLower (Utilities|String|RightChop Command (Utilities|String|Len (Variables|Default|GetcommandPrefix))))
    (:help
      (CallFunction|CommandHelp _username))
    (:ping
      (CallFunction|CommandPing _username))
    (:test
      (CallFunction|CommandTest))))

(fn CommandHelp
  (params (UserName :type String))
  (Class|TwitchChat|SendMessage (Variables|Default|GetHelpMessage)))

(fn CommandPing
  (params (UserName :type String))
  (Class|TwitchChat|SendWhisper "Pong!" UserName))

(fn CommandTest
  (bind _returnvalue (Actor|GetActorOfClass "/Game/Blueprints/GameEventManger.GameEventManger_C"))
  (Default|TriggerFunction _returnvalue))

(fn ReadSettings
  (bind _returnvalue (Class|BlueprintPathsLibrary|ProjectConfigDir))
  (bind _configfilename (Variables|Default|GetConfigFileName))
  (bind _returnvalue_2 (Utilities|String|Append _returnvalue _configfilename))
  (bind _filepath (Utilities|Struct|MakeFilePath _returnvalue_2))
  (if (Class|BlueprintPathsLibrary|FileExists _returnvalue_2)
    (bind _outjsonobject (Class|JsonBlueprintFunctionLibrary|FromFile _filepath))
    (bind (_outvalue _outvalue2 _outvalue3 _outvalue4 _outvalue5) (|Readding _outjsonobject _outjsonobject _outjsonobject _outjsonobject _outjsonobject)
      (:then_3
        (return _outvalue _outvalue2 _outvalue3 _outvalue4 _outvalue5)))
    (else
      (bind _outjsonobject_2 (Class|JsonBlueprintFunctionLibrary|FromString "{ 
    \"Token\":\"\", 
    \"Channel\":\"\", 
    \"Username\":\"\", 
    \"CommandPrefix\":\"\", 
    \"HelpMessage\":\"\" 
}"))
      (Class|JsonBlueprintFunctionLibrary|ToFile _outjsonobject_2 _filepath))))

(fn SetSettings
  (params (Token :type String) (Channel :type String) (Username :type String) (CommandPrefix :type String) (HelpMessage :type String))
  (Utilities|FlowControl|Sequence
    (:then_0
      (|Setting Token Channel Username CommandPrefix HelpMessage))
    (:then_1
      (Class|TwitchChat|ConnecttoTwitch)
      (Development|PrintString (Utilities|String|Append "Connected: " (Utilities|String|ToString(Boolean) (Variables|Default|GetbIsConnected)))))))