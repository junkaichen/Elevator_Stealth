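; BP_PikminManager keeps a squad of Pikmin spawned around the player and spends them to cast skills.
; BeginPlay spawns MaxNum Pikmin at random horizontal offsets near the player character and tracks them in PikminList.
; TriggerEvent matches an ID against SkillName, has the first Pikmin cast that skill, then drops it from the list.
; RespawnPikmin refills the squad one delayed spawn at a time, using CanRespawn to block overlapping refills.
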(event Custom|SpawnPikmin
  (bind _returnvalue (Game|SpawnActorfromClass "/Game/Blueprints/Pikmin/BP_Pikmin.BP_Pikmin_C" (Math|Transform|MakeTransform (+ (Transformation|GetActorLocation (Game|GetPlayerCharacter 0)) (Math|Vector|MakeVector (Math|Random|RandomFloatinRange -2e+02 2e+02) (Math|Random|RandomFloatinRange -2e+02 2e+02) 1.2e+02)) "0, 0, 0" "1.000000,1.000000,1.000000") "AdjustIfPossibleButAlwaysSpawn" 0 0))
  (Utilities|Array|Add (Variables|Default|GetPikminList) _returnvalue))

(event Custom|RespawnPikmin
  (if (Variables|Default|GetCanRespawn)
    (Variables|Default|SetCanRespawn false)
    (Utilities|FlowControl|Delay 1.5)
    (CallFunction|SpawnPikmin)
    (Variables|Default|SetCanRespawn true)
    (if (< (Utilities|Array|Length (Variables|Default|GetPikminList)) (Variables|Default|GetMaxNum))
      (CallFunction|RespawnPikmin))))

(event EventBeginPlay
  (|CallParentFunction)
  (for _index (range 0 (- (Variables|Default|GetMaxNum) 1))
    (CallFunction|SpawnPikmin)))

(event EventTriggerEvent
  (params (ObjId :type String))
  (for _array_element (Variables|Default|GetSkillName)
    (if (and (Utilities|Enum|Equal(Enum) ObjId _array_element) (> (Utilities|Array|Length (Variables|Default|GetPikminList)) 0))
      (Default|CastSkill (Utilities|Array|Get(acopy) (Variables|Default|GetPikminList)) _array_element)
      (Utilities|Array|RemoveIndex (Variables|Default|GetPikminList))
      (CallFunction|RespawnPikmin))))

(fn ConstructionScript
  (|CallParentFunction))