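; BP_Pikmin is a follower pawn that trails the player character and can blow itself up as a skill.
; It spawns its default controller on BeginPlay, then issues AIMoveTo from Tick whenever it is beyond follow range of the player.
; The CastSkill event switches on the skill name; Explosion prints a message, waits briefly, spawns a particle effect and destroys the actor, with no damage applied.
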(event Custom|CastSkill
  (params (SkillName :type String))
  (switch string SkillName
    (:explosion
      (Development|PrintString "Boom")
      (Utilities|FlowControl|Delay 1.0)
      (Effects|SpawnEmitteratLocation "/Game/StarterContent/Particles/P_Explosion.P_Explosion" (Transformation|GetActorLocation))
      (Actor|DestroyActor))))

(event EventBeginPlay
  (Pawn|SpawnDefaultController))

(event EventTick
  (params (DeltaSeconds :type Float%20%28single-precision%29))
  (bind _returnvalue (Game|GetPlayerCharacter 0))
  (if (> (Math|Vector|Distance(Vector) (Transformation|GetActorLocation) (Transformation|GetActorLocation _returnvalue)) 1.5e+02)
    (AI|AIMoveTo self "0, 0, 0" _returnvalue 1.5e+02 false)))

(fn ConstructionScript)