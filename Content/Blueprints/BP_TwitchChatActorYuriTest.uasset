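; Test Twitch chat bot actor that connects to a channel and turns prefixed chat commands into game actions.
; On BeginPlay it loads credentials, channel, prefix and help text from a JSON file in the config directory, or writes a blank template without connecting.
; ProcessCommand strips the prefix, answers help and ping, and forwards unrecognized commands with the user name to GameEventManger; the test command is a stub.
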(event EventBeginPlay
  (bind _returnvalue (Class|BlueprintPathsLibrary|ProjectConfigDir))
  (bind _configfilename (Variables|Default|GetConfigFileName))
  (bind _returnvalue_2 (Utilities|String|Append _returnvalue _configfilename))
  (bind _filepath (Utilities|Struct|MakeFilePath _returnvalue_2))
  (if (Class|BlueprintPathsLibrary|FileExists _returnvalue_2)
    (bind _outjsonobject (Class|JsonBlueprintFunctionLibrary|FromFile _filepath))
    (Utilities|FlowControl|Sequence
      (:then_0
        (bind _outvalue (|GetJsonField _outjsonobject "Token"))
        (Variables|Default|Settoken _outvalue)
        (bind _outvalue_2 (|GetJsonField _outjsonobject "CommandPrefix"))
        (Variables|Default|SetcommandPrefix _outvalue_2))
      (:then_1
        (bind _outvalue_3 (|GetJsonField _outjsonobject "Channel"))
        (Variables|Default|Setchannel _outvalue_3)
        (bind _outvalue_4 (|GetJsonField _outjsonobject "HelpMessage"))
        (Variables|Default|SetHelpMessage _outvalue_4))
      (:then_2
        (bind _outvalue_5 (|GetJsonField _outjsonobject "Username"))
        (Variables|Default|Setusername _outvalue_5))
      (:then_3
        (Class|TwitchChat|ConnecttoTwitch)
        (Utilities|FlowControl|Delay 5.0)
        (Development|PrintString (Utilities|String|Append "Connected: " (Utilities|String|ToString(Boolean) (Variables|Default|GetbIsConnected))))))
    (else
      (bind _outjsonobject_2 (Class|JsonBlueprintFunctionLibrary|FromString "{ 
    \"Token\":\"\", 
    \"Channel\":\"\", 
    \"Username\":\"\", 
    \"CommandPrefix\":\"\", 
    \"HelpMessage\":\"\" 
}"))
      (Class|JsonBlueprintFunctionLibrary|ToFile _outjsonobject_2 _filepath))))

(fn ConstructionScript)

(fn IsCommand
  (params (message :type String))
  (return (Utilities|String|StartsWith message (Variables|Default|GetcommandPrefix))))

(fn ProcessCommand
  (params (Command :type String) (UserName :type String))
  (bind _commandprefix (Variables|Default|GetcommandPrefix))
  (bind _username (Variables|Default|Getusername))
  (bind _returnvalue (Utilities|String|Len _commandprefix))
  (bind _returnvalue_2 (Utilities|String|RightChop Command _returnvalue))
  (bind _returnvalue_3 (Utilities|String|ToLower _returnvalue_2))
  (switch string _returnvalue_3
    (:Default
      (CallFunction|UserCommand UserName _returnvalue_3))
    (:help
      (CallFunction|CommandHelp _username))
    (:ping
      (CallFunction|CommandPing _username))
    (:test
      (CallFunction|CommandTest))))

(fn CommandHelp
  (params (UserName :type String))
  (Class|TwitchChat|SendMessage (Variables|Default|GetHelpMessage)))

(fn CommandPing
  (params (UserName :type String))
  (Class|TwitchChat|SendWhisper "Pong!" UserName))

(fn CommandTest
  (Actor|GetActorOfClass "/Game/Blueprints/GameEventManger.GameEventManger_C"))

(fn UserCommand
  (params (UserId :type String) (ObjId :type String))
  (bind _returnvalue (Actor|GetActorOfClass "/Game/Blueprints/GameEventManger.GameEventManger_C"))
  (Utilities|IsValid _returnvalue
    (:Is%20Valid
      (Default|TriggerFunctionCmd _returnvalue UserId ObjId))))