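; Door actor that swings open or shut in response to interactive events from the level's GameEventManger.
; On BeginPlay it animates to its initial Open state, then binds TriggerEvent to the manager's event.
; TriggerEvent compares object IDs, toggles Open and calls DoorMove.
; DoorMove restarts either the open or close timeline, whose value scales RotateAngle to set the door mesh's relative yaw.
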(event Custom|TriggerEvent
  (params (ObjId :type String))
  (if (Utilities|Enum|Equal(Enum) ObjId (Variables|Default|GetObjId))
    (Variables|Default|SetOpen (not (Variables|Default|GetOpen)))
    (CallFunction|DoorMove)))

(event Custom|DoorMove
  (bind _sm_door (Variables|Default|GetSM_Door))
  (bind _rotateangle (Variables|Default|GetRotateAngle))
  (if (Variables|Default|GetOpen)
    (bind _doortimer (Timeline|OpenTimer PlayFromStart)
      (:Update
        (Transformation|SetRelativeRotation _sm_door (Math|Rotator|MakeRotator 0.0 0.0 (* _doortimer _rotateangle)) false false)))
    (else
      (bind _doortimer_2 (Timeline|CloseTimer PlayFromStart)
        (:Update
          (Transformation|SetRelativeRotation _sm_door (Math|Rotator|MakeRotator 0.0 0.0 (* _rotateangle _doortimer_2)) false false))))))

(event EventBeginPlay
  (CallFunction|DoorMove)
  (bind _returnvalue (Actor|GetActorOfClass "/Game/Blueprints/Actors/GameEventManger.GameEventManger_C"))
  (bind _output_get (Variables|Default|SetGameEventManager _returnvalue))
  (Utilities|IsValid _output_get
    (:Is%20Valid
      (EventDispatchers|BindEventtoInteractiveEvent _output_get (delegate Custom|TriggerEvent)))))

(fn ConstructionScript)