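; Line-of-sight actor that follows the first actor of ClassToFollow and builds a 360-degree visibility shape around it.
; Each tick, a ring of Visibility line traces rotates and scales one ISM instance per ray to the hit distance.
; SCC2D's ortho width matches CheckRange, apparently to capture that shape as a mask.
; MPC_SightLine receives mask height, texture scale and actor location for materials, with setup also run at construction.
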(event Custom|SightTrace
  (bind _returnvalue (Transformation|GetActorLocation))
  (for _index (range 0 (- (Variables|Default|GetTraceCount) 1))
    (bind _output_get (Variables|Default|SetCurrentTraceStep _index))
    (bind (_outhit _returnvalue_2) (Collision|LineTraceByChannel _returnvalue (+ _returnvalue (* (Math|Vector|RotateVector (Transformation|GetActorForwardVector) (Math|Rotator|MakeRotator 0.0 0.0 (* (Math|Conversions|ToFloat(Integer) _output_get) (/ 3.6e+02 (Math|Conversions|ToFloat(Integer) (Variables|Default|GetTraceCount)))))) (Variables|Default|GetCheckRange))) "TraceTypeQuery1" false 0 "None" true "(R=1.000000,G=0.000000,B=0.000000,A=1.000000)" "(R=0.000000,G=1.000000,B=0.000000,A=1.000000)" 0.1))
    (Components|InstancedStaticMesh|UpdateInstanceTransform (Variables|Default|GetISM) (Variables|Default|GetCurrentTraceStep) (Math|Transform|MakeTransform (Math|Vector|SelectVector (Math|Vector|MakeVector 0.0 0.0 (Variables|Default|GetISM_HeightOffset)) "0, 0, 0" (Variables|Default|GetOffsetByHeight)) (Math|Rotator|FindLookatRotation (.TraceStart (Collision|BreakHitResult _outhit)) (.TraceEnd (Collision|BreakHitResult _outhit))) (Math|Vector|MakeVector (* (Math|Vector|VectorLength (- (Math|Vector|SelectVector (.Location (Collision|BreakHitResult _outhit)) (.TraceEnd (Collision|BreakHitResult _outhit)) _returnvalue_2) (.TraceStart (Collision|BreakHitResult _outhit)))) (Variables|Default|GetTraceHitOffset)) (* (/ 3.6e+02 (Math|Conversions|ToFloat(Integer) (Variables|Default|GetTraceCount))) (* (Math|Vector|VectorLength (- (Math|Vector|SelectVector (.Location (Collision|BreakHitResult _outhit)) (.TraceEnd (Collision|BreakHitResult _outhit)) _returnvalue_2) (.TraceStart (Collision|BreakHitResult _outhit)))) (Variables|Default|GetTraceHitOffset))) (* (Math|Vector|VectorLength (- (Math|Vector|SelectVector (.Location (Collision|BreakHitResult _outhit)) (.TraceEnd (Collision|BreakHitResult _outhit)) _returnvalue_2) (.TraceStart (Collision|BreakHitResult _outhit)))) (Variables|Default|GetTraceHitOffset)))) false true true)))

(event Custom|InitializeISM
  (Components|InstancedStaticMesh|ClearInstances (Variables|Default|GetISM))
  (for _index (range 0 (- (Variables|Default|GetTraceCount) 1))
    (Components|InstancedStaticMesh|AddInstance (Variables|Default|GetISM) (Math|Transform|MakeTransform "0, 0, 0") false))
  (CallFunction|SightTrace)
  (Variables|/Script/Engine.SceneCaptureComponent2D|SetOrthoWidth (Variables|Default|GetSCC2D) (Variables|Default|GetCheckRange))
  (Transformation|SetRelativeTransform (Variables|Default|GetSCC2D) (Math|Transform|MakeTransform (Math|Vector|MakeVector 0.0 0.0 (- (Variables|Default|GetISM_HeightOffset) 1.0)) "90.000000, 0, 0" "1.000000,-1.000000,-1.000000") false false)
  (Rendering|Material|SetScalarParameterValue "/Game/Blueprints/LineOfSight/MPC_SightLine.MPC_SightLine" "SightLineMaskHeight" (+ (.z (Transformation|GetActorLocation)) (Variables|Default|GetISM_HeightOffset) -5e+02) :!class /Script/Engine.KismetMaterialLibrary)
  (Rendering|Material|SetScalarParameterValue "/Game/Blueprints/LineOfSight/MPC_SightLine.MPC_SightLine" "SightLineTexScale" (Variables|Default|GetCheckRange) :!class /Script/Engine.KismetMaterialLibrary)
  (Rendering|Material|SetVectorParameterValue "/Game/Blueprints/LineOfSight/MPC_SightLine.MPC_SightLine" "SightLineActorLocation" (Math|Conversions|ToLinearColor(Vector) (Transformation|GetActorLocation)) :!class /Script/Engine.KismetMaterialLibrary))

(event EventBeginPlay
  (CallFunction|InitializeISM)
  (bind _outactors (Actor|GetAllActorsOfClass (Variables|Default|GetClassToFollow)))
  (Variables|Default|SetActorToFollow (Utilities|Array|Get(acopy) _outactors)))

(event EventTick
  (params (DeltaSeconds :type Float%20%28single-precision%29))
  (bind _actortofollow (Variables|Default|GetActorToFollow))
  (Utilities|IsValid _actortofollow
    (:Is%20Valid
      (Transformation|SetActorLocation (Transformation|GetActorLocation _actortofollow) false false)
      (CallFunction|SightTrace)
      (Rendering|Material|SetVectorParameterValue "/Game/Blueprints/LineOfSight/MPC_SightLine.MPC_SightLine" "SightLineActorLocation" (Math|Conversions|ToLinearColor(Vector) (Transformation|GetActorLocation)) :!class /Script/Engine.KismetMaterialLibrary))))

(fn ConstructionScript
  (CallFunction|InitializeISM))